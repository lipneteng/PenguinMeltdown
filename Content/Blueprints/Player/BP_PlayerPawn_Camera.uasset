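; BP_PlayerPawn_Camera is a player pawn Blueprint that creates the HUD and relays hotkey input to it.
; On BeginPlay it creates the HUD widget, stores a reference and adds it to the viewport.
; F8, F9 and F10 call the widget's info, restart and quit functions, and Escape closes its instructions.
; Its graphs contain no camera or movement logic.
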(event `self.ReceiveBeginPlay`
  (bind _returnvalue (`|CreateWidget` "/Game/UI/HUD.HUD_C"))
  (bind _output_get (set `self.HUDRef` _returnvalue))
  (`UserWidget.AddToViewport` _output_get 0))

(event `Key|F8`
  (params (Key :type "Key Structure" :default "AnyKey"))
  (:`Pressed`
    (`/Game/UI/HUD.CallInfo` (`self.HUDRef`))))

(event `Key|F9`
  (params (Key :type "Key Structure" :default "AnyKey"))
  (:`Pressed`
    (`/Game/UI/HUD.CallRestart` (`self.HUDRef`))))

(event `Key|F10`
  (params (Key :type "Key Structure" :default "AnyKey"))
  (:`Pressed`
    (`/Game/UI/HUD.CallQuit` (`self.HUDRef`))))

(event `Key|Escape`
  (params (Key :type "Key Structure" :default "AnyKey"))
  (:`Pressed`
    (`/Game/UI/HUD.CloseInstruction` (`self.HUDRef`))))

(fn `UserConstructionScript`)